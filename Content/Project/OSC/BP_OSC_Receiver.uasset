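; OSC receiver that runs a listening server and opens a web browser widget on BeginPlay.
; Audio FFT floats and object or last-group commands go out through separate calls, and FFT activation messages are ignored.
; Other messages go to all BPI_OSCInterface actors behind a lock, queuing while it is held.
; The mesh creator's finish event schedules next-tick execution to replay the queue in order and release the lock.
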(event Custom|OSC%20Message%20Execute
  ;[1 1 1] For debugging
  (if (Utilities|Array|IsNotEmpty (Variables|OSCReceiver|GetOSCMessagesCache))
    (bind _returnvalue (Class|OSCManager|GetOSCMessageAddress (Utilities|Array|Get(acopy) (Variables|OSCReceiver|GetOSCMessagesCache))))
    (bind _returnvalue_2 (Class|OSCManager|GetOSCAddressFullPath _returnvalue))
    (for _array_element (Variables|OSCReceiver|GetOSCControl%20Actors)
      ;[1 1 1] Reset Lock
      (Class|BPIOSCInterface|OSCMessage(Message) _array_element (Utilities|Array|Get(acopy) (Variables|OSCReceiver|GetOSCMessagesCache))))
    (Utilities|Array|RemoveIndex (Variables|OSCReceiver|GetOSCMessagesCache))
    (if (Utilities|Array|IsEmpty (Variables|OSCReceiver|GetOSCMessagesCache))
      (Variables|OSCReceiver|SetLock false :!label _label))
    (else
      (goto _label))))

(event Custom|ManagerMessage
  (params (ManagerMessage :type OSC%20Message%20Structure))
  ;[1 1 1] Message To OSC Manager
  (if (Variables|OSCReceiver|GetLock)
    (Utilities|Array|Add (Variables|OSCReceiver|GetOSCMessagesCache) ManagerMessage)
    (else
      (Variables|OSCReceiver|SetLock true)
      (for _array_element (Variables|OSCReceiver|GetOSCControl%20Actors)
        (Class|BPIOSCInterface|OSCMessage(Message) _array_element ManagerMessage)))))

(event Custom|OSC%20Message%20Received
  (params (Message :type OSC%20Message%20Structure%20%28by%20ref%29) (IPAddress :type String) (Port :type Integer))
  ;[1 1 1] Received
  (bind _returnvalue (Class|OSCManager|GetOSCMessageAddress Message))
  (bind _returnvalue_2 (Class|OSCManager|GetOSCAddressFullPath _returnvalue))
  (if (Utilities|Enum|NotEqual(Enum) _returnvalue_2 "/Activate/FFT")
    (if (Utilities|Enum|Equal(Enum) _returnvalue_2 "/Audio/FFT")
      (bind _values (Class|OSCManager|GetAllFloats Message))
      (Default|CallOnAudioFFT _values)
      (elif (or (Utilities|String|Contains _returnvalue_2 "LastGroup") (Utilities|String|Contains _returnvalue_2 "Object"))
        (Default|CallCommandforObjects Message)
        (else
          (CallFunction|ManagerMessage Message))))))

(event Custom|Execute%20Next%20Command
  ;[1 1 1] Initialize The OSC Receiver
  (Class|KismetSystemLibrary|SetTimerforNextTickDelegate (EventDispatchers|CreateEvent :!event Custom|OSC%20Message%20Execute)))

(event EventBeginPlay
  ;[1 1 1] Initialize The OSC Receiver
  (Utilities|FlowControl|Sequence
    (:then_0
      (bind _returnvalue (Class|OSCManager|CreateOSCServer "0.0.0.0" (Variables|OSCReceiver|GetPort) false true "" 0))
      (bind _output_get (Variables|OSCReceiver|SetOSCServer_Ref _returnvalue))
      (EventDispatchers|BindEventtoOnOscMessageReceived _output_get (EventDispatchers|CreateEvent :!event Custom|OSC%20Message%20Received)))
    (:then_1
      (bind _outactors (Actor|GetAllActorswithInterface "/Game/Project/OSC/BPI_OSCInterface.BPI_OSCInterface_C"))
      (Variables|OSCReceiver|SetOSCControl%20Actors _outactors))
    (:then_2
      (bind _returnvalue_2 (Actor|GetActorOfClass "/Game/Project/OSC/Blueprints/Manager/BP_OSCMesh_Creator.BP_OSCMesh_Creator_C"))
      (bind _output_get_2 (Variables|Default|SetMeshManager _returnvalue_2))
      (EventDispatchers|BindEventtoFinishCommand _output_get_2 (delegate Custom|Execute%20Next%20Command)))
    (:then_3
      (bind _returnvalue_3 (UserInterface|CreateWidget "/Game/Project/OSC/Widget/WBP_WebBrowser.WBP_WebBrowser_C" (Game|GetPlayerController 0)))
      (UserInterface|Viewport|AddtoViewport _returnvalue_3 0))
    (:then_4
      (Utilities|Array|Clear (Variables|OSCReceiver|GetOSCMessagesCache))
      (Variables|OSCReceiver|SetLock false))))

(fn ConstructionScript)
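; BP_AudioSphere is an audio visualizer that starts playing its sound when it receives the OSC address /play/music.
; On trigger it gathers and shuffles all BP_OSCCube actors, then plays the sound with a playback-percent callback.
; The callback converts progress to time, samples Constant-Q analysis, and maps each band to a cube's randomized height and shared MPC_MusicCube intensity parameters.
; A separate event, not called here, applies MI_MusicCube to those cubes.
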(event Custom|Playback%20Feedback
  (params (PlayingSoundWave :type Sound%20Wave%20Object%20Reference) (PlaybackPercent :type Float%20%28single-precision%29))
  (Variables|Audio|SetPlayTime (* PlaybackPercent (Variables|Audio|GetSoundDuration)))
  (for (_array_element _array_index) (Class|ConstantQNRT|GetNormalizedChannelConstantQatTime (Variables|Audio|GetStN_Analysis) (Variables|Audio|GetPlayTime))
    (Utilities|IsValid (Utilities|Array|Get(acopy) (Variables|Audio|GetVisualizeMusic_Cube) _array_index)
      (:Is%20Valid
        (Transformation|SetWorldScale3D (Variables|/Game/Project/OSC/Blueprints/Objects/MeshObject/BP_OSCMesh.BP_OSCMesh_C|GetStaticMesh (Utilities|Array|Get(acopy) (Variables|Audio|GetVisualizeMusic_Cube) _array_index)) (Math|Vector|MakeVector 0.5 0.5 (* _array_element (Math|Random|RandomFloatinRange 2.0 4.0))))
        (Rendering|Material|SetScalarParameterValue "/Game/Project/OSC/Materials/MPC/MPC_MusicCube.MPC_MusicCube" "WPO Intensity" (/ _array_element (Math|Random|RandomFloatinRange 2.0 7.0)) :!class /Script/Engine.KismetMaterialLibrary)
        (Rendering|Material|SetScalarParameterValue "/Game/Project/OSC/Materials/MPC/MPC_MusicCube.MPC_MusicCube" "Intensity" _array_element :!class /Script/Engine.KismetMaterialLibrary)))))

(event Custom|Get%20Cube
  (bind _outactors (Actor|GetAllActorsOfClass "/Game/Project/OSC/Blueprints/Objects/MeshObject/BP_OSCCube.BP_OSCCube_C"))
  (bind _output_get (Variables|Audio|SetVisualizeMusic_Cube _outactors))
  (Utilities|Array|Shuffle _output_get))

(event Custom|Set%20Custom%20Materials
  (for _array_element (Variables|Audio|GetVisualizeMusic_Cube)
    (Utilities|IsValid _array_element
      (:Is%20Valid
        (Rendering|Material|SetMaterial (Variables|/Game/Project/OSC/Blueprints/Objects/MeshObject/BP_OSCMesh.BP_OSCMesh_C|GetStaticMesh _array_element) 0 "/Game/Project/OSC/Materials/MI_MusicCube.MI_MusicCube")))))

(event Custom|Band
  (CallFunction|GetCube)
  (Audio|Components|Audio|SetSound (Variables|Default|GetAudio) (Variables|Audio|GetSoundSource))
  (Variables|Audio|SetSoundDuration (Variables|/Script/Engine.SoundBase|GetDuration (Variables|Audio|GetSoundSource)))
  (EventDispatchers|BindEventtoOnAudioPlaybackPercent (Variables|Default|GetAudio) (delegate Custom|Playback%20Feedback))
  (Audio|Components|Audio|Play (Variables|Default|GetAudio) 0.0))

(event EventOSCMessage
  (params (MessageContent :type OSC%20Message%20Structure))
  (bind _returnvalue (Class|OSCManager|GetOSCMessageAddress MessageContent))
  (bind _returnvalue_2 (Class|OSCManager|GetOSCAddressFullPath _returnvalue))
  (switch string _returnvalue_2
    (:/play/music
      (CallFunction|Band))))

(fn ConstructionScript)
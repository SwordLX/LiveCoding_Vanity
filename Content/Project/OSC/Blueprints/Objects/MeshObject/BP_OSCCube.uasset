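; BP_OSCCube is a cube mesh object in the OSC project that animates its appearance when spawned.
; On BeginPlay it runs the parent logic, then plays the Scale timeline, whose curve lerps the StaticMesh's world Z scale from zero to one while keeping X and Y.
; Tick and construction only call the parent, and the rotation and debug arrow and box nodes are unconnected.
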(event EventBeginPlay
  (bind _staticmesh (Variables|Default|GetStaticMesh))
  (bind _returnvalue (Transformation|GetWorldScale _staticmesh))
  (|CallParentFunction)
  (bind _curve0_1 (Timeline|Scale Play)
    (:Update
      (Transformation|SetWorldScale3D (Variables|Default|GetStaticMesh) (Math|Vector|Lerp(Vector) (Math|Vector|MakeVector (.x _returnvalue) (.y _returnvalue) 0.0) (Math|Vector|MakeVector (.x _returnvalue) (.y _returnvalue) 1.0) _curve0_1)))))

(event Collision|EventActorBeginOverlap
  (params (OtherActor :type Actor%20Object%20Reference))
  (|CallParentFunction OtherActor) ; This node is disabled and will not be called.\nDrag off pins to build functionality.
)

(event EventTick
  (params (DeltaSeconds :type Float%20%28single-precision%29))
  (|CallParentFunction DeltaSeconds))

(fn ConstructionScript
  (|CallParentFunction))
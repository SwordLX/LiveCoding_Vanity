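; OSC-controlled mesh actor that moves, rotates, spins, scales, and changes material or color from incoming commands.
; BP_OSC_Receiver delivers commands, applied on matching ID or to "LastGroup" while SpawnIteration is 1; timelines drive transform and color changes.
; An instrument command toggles binding to the receiver's audio FFT, feeding that instrument's value to an empty AudioReaction event.
; Offset plays ScaleCurve and scale plays MoveCurve, though each sets the other timeline's play rate.
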(event Custom|LevelUp
  ;[1 1 1] Every time Mesh Creator finishs construction, get "Older"
  (Math|Integer|IncrementInt (Variables|ObjectProperties|GetSpawnIteration)))

(event EventBeginPlay
  (Utilities|FlowControl|Sequence
    (:then_0
      (Variables|ObjectProperties|SetSpawnIteration 0)
      (bind _returnvalue (Actor|GetActorOfClass "/Game/Project/OSC/BP_OSC_Receiver.BP_OSC_Receiver_C"))
      (Variables|OSCMessage|SetOSC_Receiver _returnvalue)
      (bind _returnvalue_2 (Actor|GetActorOfClass "/Game/Project/OSC/Blueprints/Manager/BP_OSCMesh_Creator.BP_OSCMesh_Creator_C"))
      (Variables|OSCMessage|SetOSC_MeshCreator _returnvalue_2))
    (:then_1
      (Utilities|IsValid (Variables|OSCMessage|GetOSC_Receiver)
        (:Is%20Valid
          (EventDispatchers|BindEventtoCommandforObjects (Variables|OSCMessage|GetOSC_Receiver) (EventDispatchers|CreateEvent :!event OSCMessage)))
        (:Is%20Not%20Valid
          _))
      (Utilities|IsValid (Variables|OSCMessage|GetOSC_MeshCreator)
        (:Is%20Valid
          (EventDispatchers|BindEventtoConstructionFinish (Variables|OSCMessage|GetOSC_MeshCreator) (EventDispatchers|CreateEvent :!event Custom|LevelUp)))))))

(event EventOSCMessage
  (params (MessageContent :type OSC%20Message%20Structure))
  ;[1 1 1] Command Group
  (|CallParentFunction MessageContent)
  (if (and (Utilities|String|Contains (Variables|Default|GetOSCAddress) "LastGroup") (== (Variables|ObjectProperties|GetSpawnIteration) 1))
    (Variables|Default|SetOSCAddress (Utilities|String|Replace (Variables|Default|GetOSCAddress) "LastGroup" "Object"))
    (switch string (Variables|Default|GetOSCAddress) :!label _label
      (:/Object/offset
        (CallFunction|OffsetCommand "0, 0, 0"))
      (:/Object/direction
        (CallFunction|RotationCommand "0, 0, 0"))
      (:/Object/rotateRate
        (CallFunction|SetTickRotation))
      (:/Object/scale
        (CallFunction|ScaleCommand "0, 0, 0"))
      (:/Object/material
        (CallFunction|ChangeMaterial))
      (:/Object/color
        (CallFunction|ChangeColor))
      (:/Object/Instrument
        (CallFunction|BindFFTFunction)))
    (elif (== (CallFunction|GetFirstInteger) (Variables|ObjectProperties|GetID))
      (goto _label))))

(event EventTick
  (params (DeltaSeconds :type Float%20%28single-precision%29))
  ;[1 1 1] Rotation Rate
  (Transformation|AddActorLocalRotation (* (* (* (Variables|ObjectProperties|GetTickRotation) DeltaSeconds) (Variables|ObjectProperties|GetRotationRate)) 1e+01) false false))

(event Custom|ChangeColor
  (params (NewColor :type Color%20Structure))
  (bind _staticmesh (Variables|Default|GetStaticMesh))
  ;[1 1 1] Color Change
  (CallFunction|SetColor)
  (bind _returnvalue (Rendering|Material|CreateDynamicMaterialInstance _staticmesh 0 (Rendering|Material|GetMaterial _staticmesh 0) "None" :!class /Script/Engine.PrimitiveComponent))
  (bind _returnvalue_2 (Rendering|Material|GetVectorParameterValue _returnvalue "Color" :!class /Script/Engine.MaterialInstanceDynamic))
  (bind _colorshift (Timeline|ColorShiftCurve Play)
    (:Update
      (Rendering|Material|SetVectorParameterValue _returnvalue "Color" (Math|Color|Lerp(LinearColor) _returnvalue_2 (Variables|ObjectProperties|GetObjectColor) _colorshift) :!class /Script/Engine.MaterialInstanceDynamic))))

(event Custom|ChangeMaterial
  (params (MatID :type Integer))
  ;[1 1 1] Material Change
  (Variables|ObjectProperties|SetMaterialID MatID)
  (CallFunction|SetMaterialID)
  (switch int (Variables|ObjectProperties|GetMaterialID)
    (:0
      (Rendering|Material|SetMaterial (Variables|Default|GetStaticMesh) 0 "/Game/Project/OSC/Materials/MI_StaticMesh.MI_StaticMesh"))
    (:1
      (Rendering|Material|SetMaterial (Variables|Default|GetStaticMesh) 0 "/Game/Project/OSC/Materials/MI_Metal_Copper.MI_Metal_Copper"))
    (:2
      (Rendering|Material|SetMaterial (Variables|Default|GetStaticMesh) 0 "/Game/Project/OSC/Materials/MI_Rock_Basalt.MI_Rock_Basalt"))
    (:3
      (Rendering|Material|SetMaterial (Variables|Default|GetStaticMesh) 0 "/Game/Project/OSC/Materials/MI_MusicalScale.MI_MusicalScale"))
    (:4
      (Rendering|Material|SetMaterial (Variables|Default|GetStaticMesh) 0 "/Game/Project/OSC/Materials/MI_RainbowGrid.MI_RainbowGrid"))
    (:5
      (Rendering|Material|SetMaterial (Variables|Default|GetStaticMesh) 0 "/Game/Project/OSC/Materials/MI_Mosaic.MI_Mosaic"))
    (:6
      (Rendering|Material|SetMaterial (Variables|Default|GetStaticMesh) 0 "/Game/Project/OSC/Materials/MI_SolidColor.MI_SolidColor"))
    (:7
      (Rendering|Material|SetMaterial (Variables|Default|GetStaticMesh) 0 "/Game/Project/OSC/Materials/MI_GhostField.MI_GhostField"))
    (:8
      (Rendering|Material|SetMaterial (Variables|Default|GetStaticMesh) 0 "/Game/Project/OSC/Materials/MI_LightningCloud.MI_LightningCloud"))))

(event Custom|OffsetCommand
  (params (Value :type Vector))
  (CallFunction|SetOffsetLocation)
  (Components|Timeline|SetPlayRate (Variables|Default|GetMoveCurve) 0.5)
  (bind _moveto (Timeline|ScaleCurve Play)
    (:Update
      (Transformation|AddActorLocalOffset (Math|Vector|Lerp(Vector) "0, 0, 0" (Variables|ObjectProperties|GetOffsetLocation) _moveto) false false))))

(event Custom|RotationCommand
  (params (Value :type Rotator))
  (CallFunction|SetOffsetRotation)
  (Components|Timeline|SetPlayRate (Variables|Default|GetRotationCurve) 0.5)
  (bind _alpha (Timeline|RotationCurve Play)
    (:Update
      (Transformation|AddActorLocalRotation (Math|Rotator|Lerp(Rotator) "0, 0, 0" (Variables|ObjectProperties|GetOffsetRotation) _alpha) false false))))

(event Custom|ScaleCommand
  (params (Value :type Vector))
  (CallFunction|SetScale)
  (Components|Timeline|SetPlayRate (Variables|Default|GetScaleCurve) 0.5)
  (bind _alpha (Timeline|MoveCurve Play)
    (:Update
      (Transformation|SetRelativeScale3D (Variables|Default|GetDefaultSceneRoot) (Math|Conversions|ToVector(Float) (Math|Float|Lerp 1.0 (Variables|ObjectProperties|GetScaleValue) _alpha))))))

(event Custom|BindFFTFunction
  (bind _value (CallFunction|GetFirstString))
  (bind _returnvalue (Utilities|Enum|Equal(Enum) _value "None"))
  (if (Variables|ObjectProperties|GetbBindInstrument)
    (if _returnvalue
      (Utilities|IsValid (Variables|OSCMessage|GetOSC_Receiver)
        (:Is%20Valid
          (EventDispatchers|UnbindEventfromOnAudioFFT (Variables|OSCMessage|GetOSC_Receiver) (EventDispatchers|CreateEvent :!event Custom|AudioDataCheck))
          (Variables|ObjectProperties|SetbBindInstrument false)))
      (else
        (switch string (CallFunction|GetFirstString) :!label _label
          (:Default
            (Variables|ObjectProperties|SetInstrumentID 5 :!label _label_2))
          (:Drum
            (Variables|ObjectProperties|SetInstrumentID 0)
            (Variables|ObjectProperties|SetAudioMultiplier 6.0 :!label _label_3))
          (:Bass
            (Variables|ObjectProperties|SetInstrumentID 1)
            (goto _label_3))
          (:Piano
            (Variables|ObjectProperties|SetInstrumentID 2)
            (Variables|ObjectProperties|SetAudioMultiplier 1e+01 :!label _label_4))
          (:Vocal
            (Variables|ObjectProperties|SetInstrumentID 3)
            (goto _label_4))
          (:Harp
            (Variables|ObjectProperties|SetInstrumentID 4)
            (Variables|ObjectProperties|SetAudioMultiplier 15.0))
          (:Cymbal
            (goto _label_2)))))
    (elif (not _returnvalue)
      (Utilities|IsValid (Variables|OSCMessage|GetOSC_Receiver)
        (:Is%20Valid
          (EventDispatchers|BindEventtoOnAudioFFT (Variables|OSCMessage|GetOSC_Receiver) (EventDispatchers|CreateEvent :!event Custom|AudioDataCheck))
          (Variables|ObjectProperties|SetbBindInstrument true)
          (goto _label))))))

(event Custom|AudioDataCheck
  (params (AudioData :type Array%20of%20Floats%20%28double-precision%29))
  (if (and (Utilities|Array|IsNotEmpty AudioData) (< (Variables|ObjectProperties|GetInstrumentID) (Utilities|Array|Length AudioData)))
    (CallFunction|AudioReaction (Utilities|Array|Get(acopy) AudioData (Variables|ObjectProperties|GetInstrumentID)))))

(event Custom|AudioReaction
  (params (Value :type Float%20%28double-precision%29)))

(fn ConstructionScript)

(fn GetID
  (return (Variables|ObjectProperties|GetID)))

(fn SetID
  (params (ID :type Integer))
  (Variables|ObjectProperties|SetID ID))

(fn SetOffsetLocation
  (Variables|ObjectProperties|SetOffsetLocation (CallFunction|GetVector)))

(fn SetOffsetRotation
  (Variables|ObjectProperties|SetOffsetRotation (CallFunction|GetRotator)))

(fn SetTickRotation
  (Variables|ObjectProperties|SetTickRotation (CallFunction|GetRotationAxis))
  (Variables|ObjectProperties|SetRotationRate (CallFunction|GetFirstFloat)))

(fn SetScale
  (Variables|ObjectProperties|SetScaleValue (CallFunction|GetFirstFloat)))

(fn SetMaterialID
  (switch string (CallFunction|GetFirstString)
    (:Basic
      (Variables|ObjectProperties|SetMaterialID 0))
    (:Copper
      (Variables|ObjectProperties|SetMaterialID 1))
    (:Rock
      (Variables|ObjectProperties|SetMaterialID 2))
    (:MusicScale
      (Variables|ObjectProperties|SetMaterialID 3))
    (:RainbowGrid
      (Variables|ObjectProperties|SetMaterialID 4))
    (:Mosaic
      (Variables|ObjectProperties|SetMaterialID 5))
    (:MusicCube
      (Variables|ObjectProperties|SetMaterialID 6))
    (:GhostField
      (Variables|ObjectProperties|SetMaterialID 7))
    (:LightningCloud
      (Variables|ObjectProperties|SetMaterialID 8))))

(fn SetColor
  (bind _value (CallFunction|GetVector))
  (Variables|ObjectProperties|SetObjectColor (Math|Color|MakeColor (.x _value) (.y _value) (.z _value))))
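; BP_OSCSphere is a mesh object that reacts visually to audio values through its material.
; Each AudioReaction call creates a dynamic material instance on slot 0 of the static mesh.
; It sets AudioIntensity from the value times AudioMultiplier, and Audio_WorldOffset at five times that amount.
; A timeline that would pulse the mesh scale is present but never runs.
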(event EventBeginPlay
  (|CallParentFunction) ; This node is disabled and will not be called.\nDrag off pins to build functionality.
)

(event EventTick
  (params (DeltaSeconds :type Float%20%28single-precision%29))
  (|CallParentFunction DeltaSeconds) ; This node is disabled and will not be called.\nDrag off pins to build functionality.
)

(event EventAudioReaction
  (params (Value :type Float%20%28double-precision%29))
  (bind _staticmesh (Variables|Default|GetStaticMesh))
  (bind _audiomultiplier (Variables|Default|GetAudioMultiplier))
  (bind _returnvalue (* Value _audiomultiplier))
  (bind _returnvalue_2 (Rendering|Material|CreateDynamicMaterialInstance _staticmesh 0 (Rendering|Material|GetMaterial _staticmesh 0) "None" :!class /Script/Engine.PrimitiveComponent))
  (Rendering|Material|SetScalarParameterValue _returnvalue_2 "AudioIntensity" _returnvalue :!class /Script/Engine.MaterialInstanceDynamic)
  (Rendering|Material|SetScalarParameterValue _returnvalue_2 "Audio_WorldOffset" (* _returnvalue 5.0) :!class /Script/Engine.MaterialInstanceDynamic))

(fn ConstructionScript
  (|CallParentFunction))
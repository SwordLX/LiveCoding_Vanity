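; OSC object manager, filed under Deprecated, that spawns cube, sphere or cylinder actors from /Object/Definition messages.
; ProcessingMessage scans string keywords to set shape, ID, transform and material, deriving float-array indices from keyword positions, shifted once Location is read.
; SpawnObject then creates the BP_OSCMesh, applies ID and material, and records it in ObjectList before the location flag resets.
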(event Custom|SpawnObject
  (bind _returnvalue (Game|SpawnActorfromClass (Utilities|Select :Index (Variables|OSCObject|GetShapeSelected) :Option%200 "/Game/Project/OSC/Blueprints/Objects/MeshObject/BP_OSCCube.BP_OSCCube_C" :Option%201 "/Game/Project/OSC/Blueprints/Objects/MeshObject/BP_OSCSphere.BP_OSCSphere_C" :Option%202 "/Game/Project/OSC/Blueprints/Objects/MeshObject/BP_OSCCylinder.BP_OSCCylinder_C") (Math|Transform|MakeTransform (Variables|OSCObject|GetObjectPosition) (Variables|OSCObject|GetObjectRotation) (Math|Conversions|ToVector(Float) (Variables|OSCObject|GetObjectScalar))) "Undefined" "MultiplyWithRoot" 0 0))
  (bind _asbp_oscmesh (Utilities|Casting|CastToBP_OSCMesh _returnvalue))
  (Variables|/Game/Project/OSC/Blueprints/Objects/MeshObject/BP_OSCMesh.BP_OSCMesh_C|SetID _asbp_oscmesh (Variables|OSCObject|GetID))
  (Default|ChangeMaterial _asbp_oscmesh (Variables|OSCObject|GetMaterailAssignIndex))
  (Utilities|Array|AddUnique (Variables|OSCObject|GetObjectList) 0))

(event Custom|ResetValue
  (Variables|OSCObject|SetbAlreadySetLocation false))

(event EventBeginPlay
  (if (not (Utilities|Array|IsEmpty (Variables|OSCObject|GetObjectList)))
    (Utilities|Array|Clear (Variables|OSCObject|GetObjectList))))

(event EventOSCMessage
  (params (MessageContent :type OSC%20Message%20Structure))
  (|CallParentFunction MessageContent)
  (switch string (Variables|Default|GetOSCAddress)
    (:/Object/Definition
      (CallFunction|ProcessingMessage)
      (CallFunction|SpawnObject)
      (CallFunction|ResetValue))))

(fn ConstructionScript
  (|CallParentFunction))

(fn ProcessingMessage
  (for (_array_element _array_index) (Variables|Default|GetStringArray)
    (switch string _array_element
      (:cube
        (CallFunction|GetShapeandID))
      (:sphere
        (CallFunction|GetShapeandID 1))
      (:cylinder
        (CallFunction|GetShapeandID 2))
      (:scale
        (CallFunction|GetScalar _array_index))
      (:location
        (CallFunction|GetLocation _array_index))
      (:mat
        (CallFunction|GetMaterialIndex _array_index))
      (:rotateX
        (CallFunction|GetRotatorX _array_index))
      (:rotateY
        (CallFunction|GetRotatorY _array_index))
      (:rotateZ
        (CallFunction|GetRotatorZ _array_index)))))

(fn GetShapeandID
  (params (ShapeIndex :type Integer))
  (Variables|OSCObject|SetShapeSelected ShapeIndex)
  (bind (_value _returnvalue) (Class|OSCManager|GetInt32 (Variables|Default|GetMessage%20Content)))
  (if _returnvalue
    (Variables|OSCObject|SetID _value)))

(fn GetScalar
  (params (CommandIndex :type Integer))
  (bind _returnvalue (CallFunction|CalculateFloatIndex CommandIndex))
  (Variables|OSCObject|SetObjectScalar (Utilities|Array|Get(acopy) (Variables|Default|GetFloatArray) _returnvalue)))

(fn CalculateFloatIndex
  (params (CommandIndex :type Integer))
  (if (Variables|OSCObject|GetbAlreadySetLocation)
    (return (+ CommandIndex 1))
    (else
      (return (- CommandIndex 1)))))

(fn GetLocation
  (params (commandIndex :type Integer))
  (LocalVariables|SetIndex commandIndex)
  (LocalVariables|Setx_value (Utilities|Array|Get(acopy) (Variables|Default|GetFloatArray) (- (LocalVariables|GetIndex) 1)))
  (LocalVariables|Sety_value (Utilities|Array|Get(acopy) (Variables|Default|GetFloatArray) (LocalVariables|GetIndex)))
  (LocalVariables|Setz_value (Utilities|Array|Get(acopy) (Variables|Default|GetFloatArray) (+ (LocalVariables|GetIndex) 1)))
  (Variables|OSCObject|SetObjectPosition (Math|Vector|MakeVector (LocalVariables|Getx_value) (LocalVariables|Gety_value) (LocalVariables|Getz_value)))
  (Variables|OSCObject|SetbAlreadySetLocation true))

(fn GetMaterialIndex
  (params (commandIndex :type Integer))
  (switch string (Utilities|Array|Get(acopy) (Variables|Default|GetStringArray) (+ commandIndex 1))
    (:Basic
      (Variables|OSCObject|SetMaterailAssignIndex 0))
    (:Copper
      (Variables|OSCObject|SetMaterailAssignIndex 1))
    (:Basalt
      (Variables|OSCObject|SetMaterailAssignIndex 2))
    (:Tech
      (Variables|OSCObject|SetMaterailAssignIndex 3))))

(fn GetRotatorX
  (params (commandIndex :type Integer))
  (bind _returnvalue (CallFunction|CalculateFloatIndex commandIndex))
  (Variables|OSCObject|SetObjectRotation (Math|Rotator|MakeRotator (Utilities|Array|Get(acopy) (Variables|Default|GetFloatArray) _returnvalue) (.pitch (Variables|OSCObject|GetObjectRotation)) (.yaw (Variables|OSCObject|GetObjectRotation)))))

(fn GetRotatorY
  (params (commandIndex :type Integer))
  (bind _returnvalue (CallFunction|CalculateFloatIndex commandIndex))
  (Variables|OSCObject|SetObjectRotation (Math|Rotator|MakeRotator (.roll (Variables|OSCObject|GetObjectRotation)) (Utilities|Array|Get(acopy) (Variables|Default|GetFloatArray) _returnvalue) (.yaw (Variables|OSCObject|GetObjectRotation)))))

(fn GetRotatorZ
  (params (commandIndex :type Integer))
  (bind _returnvalue (CallFunction|CalculateFloatIndex commandIndex))
  (Variables|OSCObject|SetObjectRotation (Math|Rotator|MakeRotator (.roll (Variables|OSCObject|GetObjectRotation)) (.pitch (Variables|OSCObject|GetObjectRotation)) (Utilities|Array|Get(acopy) (Variables|Default|GetFloatArray) _returnvalue))))
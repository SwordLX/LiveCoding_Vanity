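; BP_ParticleManager is a deprecated manager that controls BP_fire particle actors through incoming OSC messages.
; OSCMessage compares the message's address path against three configured addresses to create, activate or deactivate fire.
; Creation reads the first three float arguments as a spawn location, spawns a BP_fire there, then zeroes the cached coordinates.
; Activation and deactivation toggle the Fire component on every BP_fire in the level via GetAllActorsOfClass.
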(event Custom|Create%20Fire
  (CallFunction|GetLocation)
  (Game|SpawnActorfromClass "/Game/Project/OSC/Blueprints/Objects/FXObject/BP_fire.BP_fire_C" (Math|Transform|MakeTransform (Math|Vector|MakeVector (Variables|Default|GetLocation%20X) (Variables|Default|GetLocation%20Y) (Variables|Default|GetLocation%20Z)) "0, 0, 0" "1.000000,1.000000,1.000000") "Undefined" "MultiplyWithRoot" 0 0)
  (Variables|Default|SetLocation%20X 0.0)
  (Variables|Default|SetLocation%20Y 0.0)
  (Variables|Default|SetLocation%20Z 0.0))

(event Custom|Activate%20Fire
  (bind _outactors (Actor|GetAllActorsOfClass "/Game/Project/OSC/Blueprints/Objects/FXObject/BP_fire.BP_fire_C"))
  (for _array_element _outactors
    (Components|Activation|SetActive (Variables|/Game/Project/OSC/Blueprints/Objects/FXObject/BP_fire.BP_fire_C|GetFire _array_element) true false)))

(event Custom|Deactivate%20Fire
  (bind _outactors (Actor|GetAllActorsOfClass "/Game/Project/OSC/Blueprints/Objects/FXObject/BP_fire.BP_fire_C"))
  (for _array_element _outactors
    (Components|Activation|SetActive (Variables|/Game/Project/OSC/Blueprints/Objects/FXObject/BP_fire.BP_fire_C|GetFire _array_element) false false)))

(event Custom|GetLocation
  ;[1 1 1] Get location
  (bind (_value _returnvalue) (Class|OSCManager|GetFloat (Variables|Default|GetMessage%20Content)))
  (if _returnvalue
    (Variables|Default|SetLocation%20X _value)
    (bind (_value_2 _returnvalue_2) (Class|OSCManager|GetFloat (Variables|Default|GetMessage%20Content) 1))
    (if _returnvalue_2
      (Variables|Default|SetLocation%20Y _value_2)
      (bind (_value_3 _returnvalue_3) (Class|OSCManager|GetFloat (Variables|Default|GetMessage%20Content) 2))
      (if _returnvalue_3
        (Variables|Default|SetLocation%20Z _value_3)))))

(event EventOSCMessage
  (params (MessageContent :type OSC%20Message%20Structure))
  (bind _output_get (Variables|Default|SetMessage%20Content MessageContent))
  (bind _returnvalue (Class|OSCManager|GetOSCMessageAddress _output_get))
  (bind _returnvalue_2 (Class|OSCManager|GetOSCAddressFullPath _returnvalue))
  (if (Utilities|Enum|Equal(Enum) _returnvalue_2 (Variables|Default|GetOSCAddress01))
    (CallFunction|CreateFire)
    (elif (Utilities|Enum|Equal(Enum) _returnvalue_2 (Variables|Default|GetOSCAddress02))
      (CallFunction|ActivateFire)
      (elif (Utilities|Enum|Equal(Enum) _returnvalue_2 (Variables|Default|GetOSCAddress03))
        (CallFunction|DeactivateFire)))))

(fn ConstructionScript)
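; Deprecated actor that procedurally builds patterns of instanced static meshes, with setters for mesh, material, spacing and layout.
; A looping timer adds instances along a direction that turns after each run, while a timeline grows the newest from zero height.
; When the path completes, another timer repeatedly yaws each instance by an index-scaled step.
; A separate ring mode spaces instances around a circle using the same spawn routine.
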(event Custom|LoopSpawn
  (if (> (Variables|SpawnIteration|GetSpawnIterator) 0)
    (CallFunction|CalculateSpawnLocation)
    (CallFunction|SpawnNewMesh)
    (Math|Integer|DecrementInt (Variables|SpawnIteration|GetSpawnIterator))
    (else
      ;[1 1 1] For Test
      (if (> (Variables|SpawnIteration|GetFirstRotateIterator) 0)
        (Variables|SpawnAttributes|SetCurrentSpawnDirection (Math|Vector|RotateVector (Variables|SpawnAttributes|GetCurrentSpawnDirection) (Variables|SpawnIteration|GetFirstRotator)))
        (Variables|SpawnAttributes|SetSpawnRotation (Math|Rotator|CombineRotators (Variables|SpawnAttributes|GetSpawnRotation) (Variables|SpawnIteration|GetFirstRotator)))
        (Variables|SpawnIteration|SetSpawnIterator (Variables|SpawnIteration|GetSpawnNumber))
        (Math|Integer|DecrementInt (Variables|SpawnIteration|GetFirstRotateIterator))
        (else
          (Utilities|Time|ClearandInvalidateTimerbyHandle (Variables|TimerHandle|GetSpawnTimerHandle))
          (Utilities|FlowControl|Delay 1.0)
          (CallFunction|TriggerAnim))))))

(event Custom|SpawnNewMesh
  (bind _returnvalue (Components|InstancedStaticMesh|AddInstance (Variables|Default|GetInstancedStaticMesh) (Math|Transform|MakeTransform (Variables|SpawnAttributes|GetSpawnLocation) (Variables|SpawnAttributes|GetSpawnRotation) "1.000000,1.000000,0.000000") true))
  (bind _output_get (Variables|Animation|SetmaxIndex _returnvalue))
  (bind _float_0_1_ (Timeline|SpawnCurve PlayFromStart)
    (:Update
      (Components|InstancedStaticMesh|UpdateInstanceTransform (Variables|Default|GetInstancedStaticMesh) _output_get (Math|Transform|MakeTransform (Variables|SpawnAttributes|GetSpawnLocation) (Variables|SpawnAttributes|GetSpawnRotation) (Math|Vector|Lerp(Vector) "1.000000,1.000000,0.000000" "1.000000,1.000000,1.000000" _float_0_1_)) true true false))
    (:Finished
      (CallFunction|ResetSpawnLocation))))

(event Custom|SetFirstRotator
  (params (value :type Rotator))
  (Variables|SpawnIteration|SetFirstRotator value)
  (Variables|SpawnAttributes|SetCurrentSpawnDirection (Math|Vector|RotateVector (Variables|SpawnAttributes|GetCurrentSpawnDirection) (Variables|SpawnIteration|GetFirstRotator))))

(event Custom|SetGap
  (params (value :type Float%20%28double-precision%29))
  (Variables|Initialization|SetGapLength value))

(event Custom|SetSpawnLocation
  (params (value :type Vector))
  (Variables|SpawnAttributes|SetSpawnLocation value))

(event Custom|SetMesh
  (params (value :type Integer))
  (Components|StaticMesh|SetStaticMesh (Variables|Default|GetInstancedStaticMesh) (Utilities|Select :Index value :Option%200 "/Game/Project/Assets/Mesh/CenterCube.CenterCube" :Option%201 "/Engine/BasicShapes/Sphere.Sphere" :Option%202 "/Engine/BasicShapes/Cylinder.Cylinder")))

(event Custom|SetInstanceMaterial
  (params (value :type Integer))
  (Rendering|Material|SetMaterial (Variables|Default|GetInstancedStaticMesh) 0 (Utilities|Select :Index value :Option%200 "/Game/Project/OSC/Materials/MI_StaticMesh.MI_StaticMesh" :Option%201 "/Game/Project/OSC/Materials/MI_Metal_Copper.MI_Metal_Copper" :Option%202 "/Game/Project/OSC/Materials/MI_Rock_Basalt.MI_Rock_Basalt" :Option%203 "/Game/Project/OSC/Materials/MI_Tech_Hex_Tile.MI_Tech_Hex_Tile")))

(event Custom|InstanceAnimation
  (bind _instancedstaticmesh (Variables|Default|GetInstancedStaticMesh))
  (Variables|Animation|SetIndexIterator 0)
  (while (<= (Variables|Animation|GetIndexIterator) (Variables|Animation|GetmaxIndex))
    (Components|InstancedStaticMesh|UpdateInstanceTransform _instancedstaticmesh (Variables|Animation|GetIndexIterator) (Math|Transform|MakeTransform (.location (.OutInstanceTransform (Components|InstancedStaticMesh|GetInstanceTransform _instancedstaticmesh (Variables|Animation|GetIndexIterator) false))) (Math|Rotator|CombineRotators (.rotation (.OutInstanceTransform (Components|InstancedStaticMesh|GetInstanceTransform _instancedstaticmesh (Variables|Animation|GetIndexIterator) false))) (Math|Rotator|MakeRotator 0.0 0.0 (* (Variables|Animation|GetIndexIterator) 2.0))) (.scale (.OutInstanceTransform (Components|InstancedStaticMesh|GetInstanceTransform _instancedstaticmesh (Variables|Animation|GetIndexIterator) false)))) false true false)
    (Math|Integer|IncrementInt (Variables|Animation|GetIndexIterator))))

(event Custom|TriggerAnim
  (bind _returnvalue (Utilities|Time|SetTimerbyEvent (delegate Custom|InstanceAnimation) 0.2 true))
  (Variables|TimerHandle|SetAnimationTimerHandle _returnvalue))

(event Custom|SpawnAnim
  (params (ID :type Integer))
  (bind _instancedstaticmesh (Variables|Default|GetInstancedStaticMesh))
  ;[1 1 1] Deprecated
  (bind _returnvalue (Rendering|Material|CreateDynamicMaterialInstance _instancedstaticmesh ID (Rendering|Material|GetMaterial _instancedstaticmesh 0) "None" :!class /Script/Engine.PrimitiveComponent))
  (bind _returnvalue_2 (Rendering|Material|GetScalarParameterValue _returnvalue "EmissiveIntensity" :!class /Script/Engine.MaterialInstanceDynamic))
  (bind _returnvalue_3 (Rendering|Material|GetVectorParameterValue _returnvalue "Color" :!class /Script/Engine.MaterialInstanceDynamic)))

(event Custom|TriggerSpawnTimer
  (Variables|SpawnIteration|SetSpawnIterator (Variables|SpawnIteration|GetSpawnNumber))
  (Variables|SpawnIteration|SetFirstRotateIterator (Variables|SpawnIteration|GetFirstRotateTime))
  (bind _returnvalue (Utilities|Time|SetTimerbyEvent (delegate Custom|LoopSpawn) 0.2 true 0.2))
  (Variables|TimerHandle|SetSpawnTimerHandle _returnvalue))

(event Custom|RotateSpawnDirection
  (params (rotator :type Rotator))
  (Variables|SpawnAttributes|SetCurrentSpawnDirection (Math|Vector|RotateVector (Variables|SpawnAttributes|GetCurrentSpawnDirection) rotator)))

(event Custom|SetSpawnNumber
  (params (value :type Integer))
  (Variables|SpawnIteration|SetSpawnNumber value))

(event Custom|SetFirstRotateTime
  (params (value :type Integer))
  (Variables|SpawnIteration|SetFirstRotateTime value))

(event EventBeginPlay
  (CallFunction|InitializeInstance)
  (Variables|SpawnIteration|SetSpawnIterator (Variables|SpawnIteration|GetSpawnNumber))
  (Variables|SpawnIteration|SetFirstRotateIterator (Variables|SpawnIteration|GetFirstRotateTime))
  (Variables|SpawnAttributes|SetCurrentSpawnDirection (Transformation|GetActorForwardVector))
  (Variables|SpawnAttributes|SetSpawnRotation (Transformation|GetActorRotation))
  (Variables|SpawnIteration|SetFirstRotator "0, 0, 0")
  (CallFunction|TriggerSpawnTimer))

(event Custom|TriggerSpawnRing
  (Variables|SpawnIteration|SetSpawnIterator 0)
  (Variables|SpawnAttributes|SetAngle 0.0)
  (Variables|SpawnAttributes|SetCircleCenter (Variables|SpawnAttributes|GetSpawnLocation))
  (Variables|SpawnAttributes|SetFinishRing false)
  (bind _returnvalue (Utilities|Time|SetTimerbyFunctionName 0 "SpawnRing" 0.2 true))
  (Variables|TimerHandle|SetRingTimer _returnvalue))

(event Custom|SetRadius
  (params (value :type Float%20%28double-precision%29))
  (Variables|SpawnAttributes|SetSpawnRadius value))

(event Custom|ResetSpawnLocation
  (if (Variables|SpawnAttributes|GetFinishRing)
    (Variables|SpawnAttributes|SetSpawnLocation (Variables|SpawnAttributes|GetCircleCenter))
    (Variables|SpawnAttributes|SetFinishRing false)))

(fn ConstructionScript)

(fn InitializeInstance
  (bind _instancedstaticmesh (Variables|Default|GetInstancedStaticMesh)
    (:then
      (bind _selectedmesh (Variables|Initialization|GetSelectedMesh)
        (:then
          (Variables|/Script/Engine.StaticMesh|SetStaticMaterials _selectedmesh (Variables|Initialization|GetStatic%20Materials))
          (Components|StaticMesh|SetStaticMesh _instancedstaticmesh _selectedmesh))
        (:else)))
    (:else)))

(fn CalculateSpawnLocation
  (Variables|SpawnAttributes|SetSpawnLocation (+ (Variables|SpawnAttributes|GetSpawnLocation) (* (Variables|SpawnAttributes|GetCurrentSpawnDirection) (Variables|Initialization|GetGapLength)))))

(fn CalculateOffsetLocation
  (params (DeltaTime :type Float%20%28double-precision%29) (OriginalLocation :type Vector))
  (bind _output_get (Variables|Animation|SetRunningTime (+ DeltaTime (Variables|Animation|GetRunningTime))))
  (return (+ OriginalLocation (Math|Vector|MakeVector 0.0 0.0 (* (Math|Trig|Sin(Radians) (* _output_get 0.5)) 2e+01)))))

(fn SpawnRing
  (bind _spawnradius (Variables|SpawnAttributes|GetSpawnRadius))
  (bind _circlecenter (Variables|SpawnAttributes|GetCircleCenter))
  (Variables|SpawnAttributes|SetSpawnLocation (Math|Vector|MakeVector (+ (* _spawnradius (Math|Trig|Cos(Degrees) (Variables|SpawnAttributes|GetAngle))) (.x _circlecenter)) (+ (* _spawnradius (Math|Trig|Sin(Degrees) (Variables|SpawnAttributes|GetAngle))) (.y _circlecenter)) (.z _circlecenter)))
  (CallFunction|SpawnNewMesh)
  (Math|Integer|IncrementInt (Variables|SpawnIteration|GetSpawnIterator)
    (:%20%20
      (if (== (Variables|SpawnIteration|GetSpawnIterator) (Variables|SpawnIteration|GetSpawnNumber))
        (Utilities|Time|ClearandInvalidateTimerbyHandle (Variables|TimerHandle|GetRingTimer))
        (Variables|SpawnAttributes|SetFinishRing true)
        (else
          (Variables|SpawnAttributes|SetAngle (+ (Variables|SpawnAttributes|GetAngle) (/ 3.6e+02 (Math|Conversions|ToFloat(Integer) (Variables|SpawnIteration|GetSpawnNumber))))))))))
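; OSC command manager that turns incoming OSC messages into runtime mesh creation and editing.
; Routes each address path, often via a shared CommandTag, to spawn cubes, spheres or cylinders, transform, recolor, change material, mirror about a point, or build rings.
; The first int argument is an object ID or ring count, and floats supply vectors and radius.
; Objects are found by scanning BP_OSCMesh actors, with MaxID supplying IDs for mirrored and ring copies.
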(event Custom|Create%20object
  (bind _idtag (Variables|Parameters|GetIDTag))
  ;[1 1 1] Create MeshObject
  (CallFunction|GetID)
  (if (Variables|Parameters|GetIDInput)
    (bind _valid_ (CallFunction|CheckValidID))
    (if _valid_
      (CallFunction|GetVectorValue)
      (bind _returnvalue (Game|SpawnActorfromClass (Utilities|Select :Index (Variables|Parameters|GetCommandTag) :Option%200 "/Game/Project/OSC/Blueprints/Objects/MeshObject/BP_OSCCube.BP_OSCCube_C" :Option%201 "/Game/Project/OSC/Blueprints/Objects/MeshObject/BP_OSCSphere.BP_OSCSphere_C" :Option%202 "/Game/Project/OSC/Blueprints/Objects/MeshObject/BP_OSCCylinder.BP_OSCCylinder_C") (Math|Transform|MakeTransform (CallFunction|BuildVector) "0, 0, 0" "1.000000,1.000000,1.000000") "Undefined" "MultiplyWithRoot" 0 0))
      (bind _asbp_oscmesh (Utilities|Casting|CastToBP_OSCMesh _returnvalue))
      (Default|SetID _asbp_oscmesh _idtag)
      (CallFunction|UpdateMaxID _idtag)
      (CallFunction|ResetVariable))
    (else
      (Development|PrintString (Variables|MessageOutput|GetWarningMessage01) true true "(R=0.396875,G=0.000000,B=0.000000,A=1.000000)" 4.0))))

(event Custom|ColorControl
  (bind _finalvector (CallFunction|BuildVector))
  ;[1 1 1] Color Control
  (CallFunction|GetID)
  (CallFunction|GetVectorValue)
  (bind _findobject_ (CallFunction|GetObjectwithID))
  (if _findobject_
    (Default|ChangeColor (Variables|Parameters|GetObjectWithID) (Math|Conversions|ToColor(LinearColor) (Math|Color|MakeColor (.x _finalvector) (.y _finalvector) (.z _finalvector))))
    (else
      (Development|PrintString (Utilities|String|Append (Utilities|String|ToString(Integer) (Variables|Parameters|GetIDTag)) (Variables|MessageOutput|GetWarningMessage02)) true true "(R=1.000000,G=0.043874,B=0.000000,A=1.000000)" 3.0))))

(event Custom|TransformObject
  (bind _finalvector (CallFunction|BuildVector))
  (bind _finalvector_2 (CallFunction|BuildVector))
  ;[1 1 1] Movement Control
  (CallFunction|GetID)
  (CallFunction|GetVectorValue)
  (bind _findobject_ (CallFunction|GetObjectwithID))
  (if _findobject_
    (switch int (Variables|Parameters|GetCommandTag)
      (:3
        (Default|OffsetCommand (Variables|Parameters|GetObjectWithID) _finalvector))
      (:4
        (Default|RotationCommand (Variables|Parameters|GetObjectWithID) (Math|Rotator|MakeRotator (.x _finalvector_2) (.y _finalvector_2) (.z _finalvector_2))))
      (:5
        (Default|ScaleCommand (Variables|Parameters|GetObjectWithID) _finalvector)))
    (else
      (Development|PrintString (Utilities|String|Append (Utilities|String|ToString(Integer) (Variables|Parameters|GetIDTag)) (Variables|MessageOutput|GetWarningMessage02)) true true "(R=1.000000,G=0.043874,B=0.000000,A=1.000000)" 3.0))))

(event Custom|MaterialControl
  ;[1 1 1] Change Material
  (CallFunction|GetID)
  (CallFunction|GetVectorValue)
  (bind _findobject_ (CallFunction|GetObjectwithID))
  (if _findobject_
    (Default|ChangeMaterial (Variables|Parameters|GetObjectWithID) (Variables|Parameters|GetCommandTag))
    (else
      (Development|PrintString (Utilities|String|Append (Utilities|String|ToString(Integer) (Variables|Parameters|GetIDTag)) (Variables|MessageOutput|GetWarningMessage02)) true true "(R=1.000000,G=0.043874,B=0.000000,A=1.000000)" 3.0))))

(event EventOSCMessage
  (params (MessageContent :type OSC%20Message%20Structure))
  ;[1 1 1] Handle Conmand
  (bind _output_get (Variables|MessageInput|SetMessage%20Content MessageContent))
  (bind _returnvalue (Class|OSCManager|GetOSCMessageAddress _output_get))
  (bind _returnvalue_2 (Class|OSCManager|GetOSCAddressFullPath _returnvalue))
  (switch string _returnvalue_2
    (:/create/cube
      (Variables|Parameters|SetCommandTag 0)
      (CallFunction|CreateObject :!label _label))
    (:/create/sphere
      (Variables|Parameters|SetCommandTag 1)
      (goto _label))
    (:/create/cylinder
      (Variables|Parameters|SetCommandTag 2)
      (goto _label))
    (:/color/mesh
      (CallFunction|ColorControl))
    (:/move/mesh
      (Variables|Parameters|SetCommandTag 3)
      (CallFunction|TransformObject :!label _label_2))
    (:/rotate/mesh
      (Variables|Parameters|SetCommandTag 4)
      (goto _label_2))
    (:/scale/mesh
      (Variables|Parameters|SetCommandTag 5)
      (goto _label_2))
    (:/defaultmat/mesh
      (Variables|Parameters|SetCommandTag 0)
      (CallFunction|MaterialControl :!label _label_3))
    (:/metalmat/mesh
      (Variables|Parameters|SetCommandTag 1)
      (goto _label_3))
    (:/rockmat/mesh
      (Variables|Parameters|SetCommandTag 2)
      (goto _label_3))
    (:/techmat/mesh
      (Variables|Parameters|SetCommandTag 3)
      (goto _label_3))
    (:/mirror/mesh
      (CallFunction|MirrorMesh))
    (:/circle/cube
      (Variables|Parameters|SetCommandTag 0)
      (CallFunction|CreateMeshCircle :!label _label_4))
    (:/circle/sphere
      (Variables|Parameters|SetCommandTag 1)
      (goto _label_4))
    (:/circle/cylinder
      (Variables|Parameters|SetCommandTag 2)
      (goto _label_4))))

(event Custom|MirrorMesh
  (CallFunction|GetVectorValue)
  (Variables|Parameters|SetMirrorPosition (CallFunction|BuildVector))
  (CallFunction|SetMirrorProperties)
  (CallFunction|ResetVariable))

(event Custom|SetCircleProperties
  (CallFunction|GetID)
  (Variables|Parameters|SetCirculNum (Variables|Parameters|GetIDTag))
  (CallFunction|GetVectorValue)
  (Variables|Parameters|SetCenterPosition (CallFunction|BuildVector))
  (Variables|Parameters|SetCircleRadius (CallFunction|GetCircleRadius)))

(event Custom|CreateMeshCircle
  (CallFunction|SetCircleProperties)
  (CallFunction|CreateMeshinCircle))

(event Custom|SetMirrorProperties
  (bind _mirrorposition (Variables|Parameters|GetMirrorPosition))
  (bind _objectwithid (Variables|Parameters|GetObjectWithID))
  (bind _returnvalue (Transformation|GetActorLocation _objectwithid))
  ;[1 1 1] Mirror Create
  (CallFunction|GetID)
  (CallFunction|GetObjectwithID)
  (bind _returnvalue_2 (Game|SpawnActorfromClass (Utilities|GetClass _objectwithid) (Math|Transform|MakeTransform (Math|Vector|MakeVector (- (* (.x _mirrorposition) 2.0) (.x _returnvalue)) (- (* (.y _mirrorposition) 2.0) (.y _returnvalue)) (- (* (.z _mirrorposition) 2.0) (.z _returnvalue))) "0, 0, 0" "1.000000,1.000000,1.000000") "Undefined" "MultiplyWithRoot" 0 0))
  (Default|SetID _returnvalue_2 (CallFunction|AutoSetID))
  (Development|PrintString "\"finish mirror\"" true true "(R=0.000000,G=0.660000,B=1.000000,A=1.000000)" 5.0))

(event Custom|GetID
  ;[1 1 1] Get Object's ID
  (bind (_value _returnvalue) (Class|OSCManager|GetInt32 (Variables|MessageInput|GetMessage%20Content)))
  (Variables|Parameters|SetIDTag _value)
  (if _returnvalue
    (Variables|Parameters|SetIDInput true)
    (else
      (Variables|Parameters|SetIDInput false))))

(event Custom|GetVectorValue
  (bind _floatinput (Variables|Parameters|GetFloatInput))
  ;[1 1 1] Set Vector
  (Utilities|Array|Clear (Variables|Parameters|GetFloatInput))
  (bind _values (Class|OSCManager|GetAllFloats (Variables|MessageInput|GetMessage%20Content)))
  (for _array_element _values
    (Utilities|Array|Add _floatinput _array_element))
  (Utilities|Array|Add _floatinput 0.0))

(event Custom|ResetVariable
  ;[1 1 1] Reset Vector
)

(fn ConstructionScript)

(fn CheckValidID
  (bind _outactors (Actor|GetAllActorsOfClass "/Game/Project/OSC/Blueprints/Objects/MeshObject/BP_OSCMesh.BP_OSCMesh_C"))
  (for _array_element _outactors
    (if (== (Default|GetID _array_element) (Variables|Parameters|GetIDTag))
      (Development|PrintString "The Input ID is occupied" true true "(R=1.000000,G=0.000000,B=0.023192,A=1.000000)" 5.0)
      (return false)))
  (return true))

(fn GetObjectwithID
  (bind _outactors (Actor|GetAllActorsOfClass "/Game/Project/OSC/Blueprints/Objects/MeshObject/BP_OSCMesh.BP_OSCMesh_C"))
  (bind _array_element (Utilities|Array|ForEachLoopwithBreak _outactors)
    (:LoopBody
      (if (== (Default|GetID _array_element) (Variables|Parameters|GetIDTag))
        (Variables|Parameters|SetObjectWithID _array_element)
        (return true)))
    (:Completed
      (return false))))

(fn CheckOccupyID
  (params (ID :type Integer))
  (Variables|Parameters|SetIDTag ID)
  (bind _valid_ (CallFunction|CheckValidID))
  (if _valid_
    (return false)
    (else
      (return true))))

(fn CreateMeshinCircle
  (bind _centerposition (Variables|Parameters|GetCenterPosition))
  (bind _circleradius (Variables|Parameters|GetCircleRadius))
  (if (> (Variables|Parameters|GetCirculNum) 0)
    (while (< (LocalVariables|Getiteration) (Variables|Parameters|GetCirculNum))
      (bind _returnvalue (Game|SpawnActorfromClass (Utilities|Select :Index (Variables|Parameters|GetCommandTag) :Option%200 "/Game/Project/OSC/Blueprints/Objects/MeshObject/BP_OSCCube.BP_OSCCube_C" :Option%201 "/Game/Project/OSC/Blueprints/Objects/MeshObject/BP_OSCSphere.BP_OSCSphere_C" :Option%202 "/Game/Project/OSC/Blueprints/Objects/MeshObject/BP_OSCCylinder.BP_OSCCylinder_C") (Math|Transform|MakeTransform (Math|Vector|MakeVector (+ (* _circleradius (Math|Trig|Cos(Degrees) (LocalVariables|GetAngle))) (.x _centerposition)) (+ (* (Math|Trig|Sin(Degrees) (LocalVariables|GetAngle)) _circleradius) (.y _centerposition)) (.z _centerposition)) "0, 0, 0" "1.000000,1.000000,1.000000") "Undefined" "MultiplyWithRoot" 0 0))
      (bind _asbp_oscmesh (Utilities|Casting|CastToBP_OSCMesh _returnvalue))
      (Default|SetID _asbp_oscmesh (CallFunction|AutoSetID))
      (LocalVariables|SetAngle (+ (LocalVariables|GetAngle) (/ 3.6e+02 (Math|Conversions|ToFloat(Integer) (Variables|Parameters|GetCirculNum)))))
      (Math|Integer|IncrementInt (LocalVariables|Getiteration)))))

(fn AutoSetID
  (bind _result (Math|Integer|IncrementInt (Variables|Parameters|GetMaxID))
    (:%20%20
      (return _result))))

(fn UpdateMaxID
  (params (ID :type Integer))
  (if (> ID (Variables|Parameters|GetMaxID))
    (Variables|Parameters|SetMaxID ID)))

(fn BuildVector
  (bind _floatinput (Variables|Parameters|GetFloatInput))
  (if (>= (Utilities|Array|Length (Variables|Parameters|GetFloatInput)) 3)
    (return (Math|Vector|MakeVector (Utilities|Array|Get(acopy) _floatinput) (Utilities|Array|Get(acopy) _floatinput 1) (Utilities|Array|Get(acopy) _floatinput 2)))
    (else
      (return "0, 0, 0"))))

(fn GetCircleRadius
  (bind _floatinput (Variables|Parameters|GetFloatInput))
  (if (< (Utilities|Array|Length _floatinput) 4)
    (return 2e+02)
    (else
      (return (Utilities|Array|Get(acopy) _floatinput 3)))))
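; BP_OSCManagerBase is an OSC manager base that unpacks incoming OSC messages into usable values.
; The OSCMessage event stores the message and its address path, then refills integer, float and string arrays from the arguments.
; Getters return first values or a vector with fallback defaults, with float and vector reads falling back to integers when no floats exist.
; Rotator and rotation axis getters use the first string (X/Y/Z) to choose the axis.
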(event EventOSCMessage
  (params (MessageContent :type OSC%20Message%20Structure))
  (bind _output_get (Variables|OSCMessage|SetMessage%20Content MessageContent))
  (OSCManagerBase|AddresstoString _output_get)
  (Utilities|Array|Clear (Variables|OSCMessage|GetIntegerArray))
  (Utilities|Array|Clear (Variables|OSCMessage|GetFloatArray))
  (Utilities|Array|Clear (Variables|OSCMessage|GetStringArray))
  (bind _values (Class|OSCManager|GetAllInt32s (Variables|OSCMessage|GetMessage%20Content)))
  (Variables|OSCMessage|SetIntegerArray _values)
  (bind _values_2 (Class|OSCManager|GetAllFloats (Variables|OSCMessage|GetMessage%20Content)))
  (Variables|OSCMessage|SetFloatArray _values_2)
  (bind _values_3 (Class|OSCManager|GetAllStrings (Variables|OSCMessage|GetMessage%20Content)))
  (Variables|OSCMessage|SetStringArray _values_3))

(fn ConstructionScript)

(fn AddresstoString
  (params (OSC%20Messager :type OSC%20Message%20Structure))
  (bind _returnvalue (Class|OSCManager|GetOSCMessageAddress OSC%20Messager))
  (bind _returnvalue_2 (Class|OSCManager|GetOSCAddressFullPath _returnvalue))
  (Variables|OSCMessage|SetOSCAddress _returnvalue_2))

(fn GetFirstInteger
  (bind _integerarray (Variables|OSCMessage|GetIntegerArray))
  (if (Utilities|Array|IsEmpty _integerarray)
    (return -1000)
    (else
      (return (Utilities|Array|Get(acopy) _integerarray)))))

(fn GetFirstFloat
  (bind _integerarray (Variables|OSCMessage|GetIntegerArray))
  (bind _floatarray (Variables|OSCMessage|GetFloatArray))
  (if (Utilities|Array|IsEmpty _floatarray)
    (if (Utilities|Array|IsEmpty _integerarray)
      (return 0.0)
      (else
        (return (Math|Conversions|ToFloat(Integer) (Utilities|Array|Get(acopy) _integerarray)))))
    (else
      (return (Utilities|Array|Get(acopy) _floatarray)))))

(fn GetFirstString
  (bind _stringarray (Variables|OSCMessage|GetStringArray))
  (if (Utilities|Array|IsEmpty _stringarray)
    (return "NULL")
    (else
      (return (Utilities|Array|Get(acopy) _stringarray)))))

(fn GetVector
  (bind _floatarray (Variables|OSCMessage|GetFloatArray))
  (bind _integerarray (Variables|OSCMessage|GetIntegerArray))
  (if (Utilities|Array|IsEmpty (Variables|OSCMessage|GetFloatArray))
    (if (Utilities|Array|IsEmpty (Variables|OSCMessage|GetIntegerArray))
      (return "0, 0, 0")
      (elif (>= (Utilities|Array|Length (Variables|OSCMessage|GetIntegerArray)) 3)
        (return (Math|Vector|MakeVector (Math|Conversions|ToFloat(Integer) (Utilities|Array|Get(acopy) _integerarray)) (Math|Conversions|ToFloat(Integer) (Utilities|Array|Get(acopy) _integerarray 1)) (Math|Conversions|ToFloat(Integer) (Utilities|Array|Get(acopy) _integerarray 2))))
        (else
          (return "0, 0, 0"))))
    (elif (>= (Utilities|Array|Length (Variables|OSCMessage|GetFloatArray)) 3)
      (return (Math|Vector|MakeVector (Utilities|Array|Get(acopy) _floatarray) (Utilities|Array|Get(acopy) _floatarray 1) (Utilities|Array|Get(acopy) _floatarray 2)))
      (else
        (return "0, 0, 0")))))

(fn GetRotator
  (switch string (OSCManagerBase|GetFirstString)
    (:Default
      (return "0, 0, 0"))
    (:X
      (return (Math|Rotator|MakeRotator (OSCManagerBase|GetFirstFloat) 0.0 0.0)))
    (:Y
      (return (Math|Rotator|MakeRotator 0.0 (OSCManagerBase|GetFirstFloat) 0.0)))
    (:Z
      (return (Math|Rotator|MakeRotator 0.0 0.0 (OSCManagerBase|GetFirstFloat))))))

(fn GetRotationAxis
  (switch string (OSCManagerBase|GetFirstString)
    (:X
      (return "0.000000,0.000000,1.000000"))
    (:Y
      (return "1.000000,0.000000,0.000000"))
    (:Z
      (return "0.000000,1.000000,0.000000"))))
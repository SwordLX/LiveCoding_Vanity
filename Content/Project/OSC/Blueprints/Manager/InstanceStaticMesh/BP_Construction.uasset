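; Procedural builder actor that spawns a chain of BP_OSCCube actors one at a time on a looping timer, starting at its own transform.
; Each new cube is offset along the previous cube's forward vector by twice its bounds extent and copies its rotation.
; Nested countdowns turn the newest cube by primary and secondary rotation offsets to bend the path, optionally reversing the secondary offset after primary turns, and clear the timer when exhausted.
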(event Custom|Construct
  (Variables|Default|GetControlMesh
    (:then
      (bind _returnvalue (CallFunction|CalculateTransform))
      (bind _returnvalue_2 (CallFunction|SpawnMesh (.location _returnvalue) (.rotation _returnvalue)))
      (Variables|Default|SetControlMesh _returnvalue_2)
      (CallFunction|CheckCondition))
    (:else)))

(event Custom|BuildTimer
  (bind _returnvalue (Utilities|Time|SetTimerbyEvent (delegate Custom|Construct) 0.1 true))
  (Variables|Default|SetConstructionTimer _returnvalue))

(event Custom|CheckCondition
  (Math|Integer|DecrementInt (Variables|Default|GetForwardIteration)
    (:%20%20
      (if (<= (Variables|Default|GetForwardIteration) 0)
        (if (<= (Variables|Default|GetRotateIteration) 0)
          (if (<= (Variables|Default|GetSecondRotateIteration) 0)
            (Utilities|Time|ClearandInvalidateTimerbyHandle (Variables|Default|GetConstructionTimer))
            (else
              (Transformation|AddActorLocalRotation (Variables|Default|GetControlMesh) (Variables|Default|GetSecondRotationOffset) false false)
              (Math|Integer|DecrementInt (Variables|Default|GetSecondRotateIteration)
                (:%20%20
                  (Variables|Default|SetRotateIteration (Variables|Default|GetRotateMaxTime))
                  (Variables|Default|SetForwardIteration (Variables|Default|GetSecondForwardMaxTime))))))
          (else
            (Transformation|AddActorLocalRotation (Variables|Default|GetControlMesh) (Variables|Default|GetRotationOffset) false false)
            (Math|Integer|DecrementInt (Variables|Default|GetRotateIteration)
              (:%20%20
                (Variables|Default|SetForwardIteration (Variables|Default|GetForwardMaxTime))
                (if (Variables|Default|GetbShouldReset)
                  (Transformation|AddActorLocalRotation (Variables|Default|GetControlMesh) (* (Variables|Default|GetSecondRotationOffset) -1.0) false false))))))))))

(event EventBeginPlay
  (bind _returnvalue (CallFunction|SpawnMesh (Transformation|GetActorLocation) (Transformation|GetActorRotation)))
  (Variables|Default|SetControlMesh _returnvalue)
  (Variables|Default|SetForwardIteration (Variables|Default|GetForwardMaxTime))
  (Variables|Default|SetRotateIteration (Variables|Default|GetRotateMaxTime))
  (Variables|Default|SetSecondRotateIteration (Variables|Default|GetSecondRotateMaxTime))
  (CallFunction|BuildTimer))

(fn ConstructionScript)

(fn SpawnMesh
  (params (location :type Vector) (rotation :type Rotator))
  (bind _returnvalue (Game|SpawnActorfromClass "/Game/Project/OSC/Blueprints/Objects/MeshObject/BP_OSCCube.BP_OSCCube_C" (Math|Transform|MakeTransform location rotation "1.000000,1.000000,1.000000") "Undefined" "MultiplyWithRoot" 0 0))
  (return _returnvalue))

(fn CalculateTransform
  (bind _controlmesh (Variables|Default|GetControlMesh))
  (bind _controlmesh_2 (Variables|Default|GetControlMesh))
  (return (Math|Transform|MakeTransform (+ (* (Transformation|GetActorForwardVector _controlmesh) (* (.BoxExtent (Collision|GetActorBounds _controlmesh true false)) 2.0)) (Transformation|GetActorLocation _controlmesh_2)) (Transformation|GetActorRotation _controlmesh_2) (Transformation|GetActorScale3D _controlmesh_2))))
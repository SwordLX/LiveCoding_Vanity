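; OSC-driven builder actor that spawns cube, sphere, cylinder or plane BP_OSCMesh actors in lines and rings.
; OSCMessage routes addresses to setters for shape, material, color, gap, position and rotation, or to construction events.
; Looping timers spawn one mesh per tick, stepping along the actor's forward vector or around a circle, optionally rotating between rows.
; Each mesh receives an incrementing ID; construction commands signal completion only after their timer finishes.
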(event Custom|SpawnOSCMesh
  ;[1 1 1] SpawnObject
  (bind _returnvalue (Game|SpawnActorfromClass (Utilities|Select :Index (Variables|ObjectProperties|GetShapeID) :Option%200 "/Game/Project/OSC/Blueprints/Objects/MeshObject/BP_OSCCube.BP_OSCCube_C" :Option%201 "/Game/Project/OSC/Blueprints/Objects/MeshObject/BP_OSCSphere.BP_OSCSphere_C" :Option%202 "/Game/Project/OSC/Blueprints/Objects/MeshObject/BP_OSCCylinder.BP_OSCCylinder_C" :Option%203 "/Game/Project/OSC/Blueprints/Objects/MeshObject/BP_OSCPlane.BP_OSCPlane_C") (Math|Transform|MakeTransform (Variables|ObjectProperties|GetObjectLocation) (Transformation|GetActorRotation) (Variables|ObjectProperties|GetObjectScale)) "Undefined" "MultiplyWithRoot" 0 0))
  (bind _asbp_oscmesh (Utilities|Casting|CastToBP_OSCMesh _returnvalue))
  (Default|ChangeMaterial _asbp_oscmesh (Variables|ObjectProperties|GetMaterialID))
  (if (Variables|ObjectProperties|GetbSetColor)
    (Default|ChangeColor _asbp_oscmesh (Math|Conversions|ToColor(LinearColor) (Variables|ObjectProperties|GetObjectColor))))
  (Default|SetID _asbp_oscmesh (Variables|SpawnIteration|GetAvailableID))
  (Math|Integer|IncrementInt (Variables|SpawnIteration|GetAvailableID)))

(event EventOSCMessage
  (params (MessageContent :type OSC%20Message%20Structure))
  ;[1 1 1] Add Command
  (|CallParentFunction MessageContent)
  (switch string (Variables|Default|GetOSCAddress)
    (:Default
      (Default|CallFinishCommand))
    (:/move/position
      (ObjectProperties|SetObjectLocation)
      (Default|CallFinishCommand :!label _label))
    (:/set/material
      (Variables|ObjectProperties|SetbSetColor false)
      (ObjectProperties|SetMeshMaterial)
      (goto _label))
    (:/rotate/direction
      (CallFunction|RotateController)
      (CallFunction|UpdateSpawnDirection)
      (goto _label))
    (:/set/mesh
      (ObjectProperties|SetMesh)
      (goto _label))
    (:/set/gaplength
      (CallFunction|SetGapLength)
      (goto _label))
    (:/forward/create
      (CallFunction|ForwardConstruction))
    (:/backward/create
      (CallFunction|BackwardConstruction))
    (:/leftward/create
      (CallFunction|LeftwardConstruction))
    (:/rightward/create
      (CallFunction|RightwardConstruction))
    (:/downward/create
      (CallFunction|DownwardConstruction))
    (:/upward/create
      (CallFunction|UpwardConstruction))
    (:/create/circle
      (CallFunction|ResetValue)
      (CallFunction|SetCircleProperties)
      (CallFunction|TriggerConstructOSCMeshinRing))
    (:/construct/direction
      (CallFunction|ResetValue)
      (CallFunction|SetConstructionProperties)
      (CallFunction|TriggerConstruction))
    (:/set/color
      (CallFunction|SetColor)
      (goto _label))
    (:/offset/X
      (CallFunction|OffsetSpawnLocation)
      (Default|CallFinishCommand :!label _label_2))
    (:/offset/Y
      (CallFunction|OffsetSpawnLocation 1)
      (goto _label_2))
    (:/offset/Z
      (CallFunction|OffsetSpawnLocation 2)
      (goto _label_2))))

(event EventBeginPlay
  (Variables|SpawnIteration|SetSpawnDirection (Transformation|GetActorForwardVector)))

(event Custom|TriggerConstruction
  ;[1 1 1] Spawn Multiple OSC Meshes
  (Variables|SpawnIteration|SetSpawnIteration 0)
  (Variables|SpawnIteration|SetRotationIteration 0)
  (bind _returnvalue (Utilities|Time|SetTimerbyEvent (delegate Custom|ConstructMultipleMeshes) 0.2 true))
  (Variables|TimerHandle|SetSpawnTimerHandle _returnvalue))

(event Custom|ConstructMultipleMeshes
  ;[1 1 1] Spawn Multiple OSC Meshes
  (if (< (Variables|SpawnIteration|GetSpawnIteration) (Variables|SpawnIteration|GetSpawnNumber))
    (CallFunction|CalculateNewSpawnLocation)
    (CallFunction|SpawnOSCMesh)
    (Math|Integer|IncrementInt (Variables|SpawnIteration|GetSpawnIteration))
    (elif (< (Variables|SpawnIteration|GetRotationIteration) (Variables|SpawnIteration|GetRotationTimes))
      (Variables|SpawnIteration|SetSpawnIteration 0)
      (CallFunction|RotateController)
      (CallFunction|UpdateSpawnDirection)
      (Math|Integer|IncrementInt (Variables|SpawnIteration|GetRotationIteration))
      (else
        (CallFunction|ResetValue)
        (Utilities|Time|ClearandInvalidateTimerbyHandle (Variables|TimerHandle|GetSpawnTimerHandle))
        (Default|CallConstructionFinish)
        (Default|CallFinishCommand)))))

(event Custom|SpawnOSCMeshInRing
  ;[1 1 1] Spawn Objects in a Circle
  (if (< (Variables|SpawnIteration|GetSpawnIteration) (Variables|SpawnIteration|GetSpawnNumber))
    (CallFunction|CalculateSpawnLocationinRing)
    (CallFunction|SpawnOSCMesh)
    (Math|Integer|IncrementInt (Variables|SpawnIteration|GetSpawnIteration)
      (:%20%20
        (Variables|SpawnIteration|SetAngleIteration (+ (Variables|SpawnIteration|GetAngleIteration) (/ 3.6e+02 (Math|Conversions|ToFloat(Integer) (Variables|SpawnIteration|GetSpawnNumber)))))))
    (else
      (Variables|ObjectProperties|SetObjectLocation (Variables|SpawnIteration|GetCenterPosition))
      (Utilities|Time|ClearandInvalidateTimerbyHandle (Variables|TimerHandle|GetSpawnRingTimerHandle))
      (CallFunction|ResetValue)
      (Default|CallConstructionFinish)
      (Default|CallFinishCommand))))

(event Custom|TriggerConstructOSCMeshInRing
  ;[1 1 1] Spawn Objects in a Circle
  (Variables|SpawnIteration|SetSpawnIteration 0)
  (Variables|SpawnIteration|SetSpawnIteration 0)
  (Variables|SpawnIteration|SetAngleIteration 0.0)
  (Variables|SpawnIteration|SetCenterPosition (Variables|ObjectProperties|GetObjectLocation))
  (bind _returnvalue (Utilities|Time|SetTimerbyEvent (delegate Custom|SpawnOSCMeshInRing) 0.1 true))
  (Variables|TimerHandle|SetSpawnRingTimerHandle _returnvalue))

(event Custom|ForwardConstruction
  ;[1 1 1] directional Spawn
  (CallFunction|ResetValue)
  (CallFunction|SetSpawnNumber)
  (CallFunction|TriggerConstruction))

(event Custom|LeftwardConstruction
  ;[1 1 1] directional Spawn
  (CallFunction|TurnDirection "0.000000,-90.000000,0.000000")
  (CallFunction|ForwardConstruction))

(event Custom|RightwardConstruction
  ;[1 1 1] directional Spawn
  (CallFunction|TurnDirection "0.000000,90.000000,0.000000")
  (CallFunction|ForwardConstruction))

(event Custom|BackwardConstruction
  ;[1 1 1] directional Spawn
  (CallFunction|TurnDirection "0.000000,180.000000,0.000000")
  (CallFunction|ForwardConstruction))

(event Custom|UpwardConstruction
  ;[1 1 1] directional Spawn
  (CallFunction|TurnDirection "90.000000,0.000000,0.000000")
  (CallFunction|ForwardConstruction))

(event Custom|DownwardConstruction
  ;[1 1 1] directional Spawn
  (CallFunction|TurnDirection "-90.000000,0.000000,0.000000")
  (CallFunction|ForwardConstruction))

(fn ConstructionScript
  (|CallParentFunction))

(fn SetMesh
  (switch string (CallFunction|GetFirstString)
    (:Cube
      (Variables|ObjectProperties|SetShapeID 0))
    (:Sphere
      (Variables|ObjectProperties|SetShapeID 1))
    (:Cylinder
      (Variables|ObjectProperties|SetShapeID 2))
    (:Plane
      (Variables|ObjectProperties|SetShapeID 3))))

(fn SetMeshMaterial
  (switch string (CallFunction|GetFirstString)
    (:Basic
      (Variables|ObjectProperties|SetMaterialID 0))
    (:Copper
      (Variables|ObjectProperties|SetMaterialID 1))
    (:Rock
      (Variables|ObjectProperties|SetMaterialID 2))
    (:MusicScale
      (Variables|ObjectProperties|SetMaterialID 3))
    (:RainbowGrid
      (Variables|ObjectProperties|SetMaterialID 4))
    (:Mosaic
      (Variables|ObjectProperties|SetMaterialID 5))
    (:MusicCube
      (Variables|ObjectProperties|SetMaterialID 6))
    (:GhostField
      (Variables|ObjectProperties|SetMaterialID 7))
    (:LightningCloud
      (Variables|ObjectProperties|SetMaterialID 8))
    (:Random
      (Variables|ObjectProperties|SetMaterialID (Math|Random|RandomIntegerinRange 0 8)))))

(fn GetScale
  (return (Math|Conversions|ToVector(Float) (CallFunction|GetFirstFloat))))

(fn SetObjectLocation
  (Variables|ObjectProperties|SetObjectLocation (CallFunction|GetVector)))

(fn SetObjectScale
  (Variables|ObjectProperties|SetObjectScale (CallFunction|GetScale)))

(fn SetGapLength
  (bind _value (CallFunction|GetFirstFloat))
  (if (< _value 0.0)
    (Variables|SpawnIteration|SetGapLength (Math|Conversions|ToFloat(Integer) (CallFunction|GetFirstInteger)))
    (else
      (Variables|SpawnIteration|SetGapLength _value))))

(fn RotateController
  (Transformation|AddActorLocalRotation (CallFunction|GetRotator) false false))

(fn SetSpawnNumber
  (Variables|SpawnIteration|SetSpawnNumber (CallFunction|GetFirstInteger)))

(fn CalculateNewSpawnLocation
  (Variables|ObjectProperties|SetObjectLocation (+ (Variables|ObjectProperties|GetObjectLocation) (* (Variables|SpawnIteration|GetSpawnDirection) (Variables|SpawnIteration|GetGapLength)))))

(fn UpdateSpawnDirection
  (Variables|SpawnIteration|SetSpawnDirection (Transformation|GetActorForwardVector)))

(fn CalculateSpawnLocationinRing
  (bind _circleradius (Variables|SpawnIteration|GetCircleRadius))
  (bind _angleiteration (Variables|SpawnIteration|GetAngleIteration))
  (Variables|ObjectProperties|SetObjectLocation (+ (Math|Vector|MakeVector (* _circleradius (Math|Trig|Cos(Degrees) _angleiteration)) (* _circleradius (Math|Trig|Sin(Degrees) _angleiteration)) 0.0) (Variables|SpawnIteration|GetCenterPosition))))

(fn ResetValue
  (Variables|SpawnIteration|SetSpawnNumber 0)
  (Variables|SpawnIteration|SetRotationTimes 0)
  (Variables|SpawnIteration|SetAngleIteration 0.0))

(fn SetCircleProperties
  (Variables|SpawnIteration|SetCircleRadius (CallFunction|GetFirstFloat))
  (Variables|SpawnIteration|SetSpawnNumber (CallFunction|GetFirstInteger)))

(fn SetConstructionProperties
  (bind _floatarray (Variables|Default|GetFloatArray))
  (Variables|SpawnIteration|SetRotationTimes (CallFunction|GetFirstInteger))
  (Variables|SpawnIteration|SetSpawnNumber (Utilities|Array|Get(acopy) (Variables|Default|GetIntegerArray) 1))
  (if (>= (Utilities|Array|Length _floatarray) 2)
    (Variables|SpawnIteration|SetGapLength (Utilities|Array|Get(acopy) _floatarray 1))))

(fn SetColor
  (bind _value (CallFunction|GetVector))
  (Variables|ObjectProperties|SetbSetColor true)
  (Variables|ObjectProperties|SetObjectColor (Math|Color|MakeColor (.x _value) (.y _value) (.z _value))))

(fn TurnDirection
  (params (Input :type Rotator))
  (Transformation|SetActorRotation Input)
  (CallFunction|UpdateSpawnDirection))

(fn OffsetSpawnLocation
  (params (AxizFlag :type Integer))
  (switch int AxizFlag
    (:0
      (LocalVariables|SetHelperVector "1.000000,0.000000,0.000000"))
    (:1
      (LocalVariables|SetHelperVector "0.000000,1.000000,0.000000"))
    (:2
      (LocalVariables|SetHelperVector "0.000000,0.000000,1.000000")))
  (Variables|ObjectProperties|SetObjectLocation (+ (Variables|ObjectProperties|GetObjectLocation) (* (CallFunction|GetFirstFloat) (LocalVariables|GetHelperVector)))))